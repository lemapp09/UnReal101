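; BP_MasterBoulder is a configurable boulder actor that places one of several cliff or rock pile meshes in the level.
; The Construction Script switches on the BoulderType variable to set the Boulder component's static mesh and matching material instance.
; It also resizes the Box component's extent to suit the chosen variant.
; The event graph holds no runtime logic.
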(event EventBeginPlay)

(event Collision|EventActorBeginOverlap
  (params (OtherActor :type Actor%20Object%20Reference)))

(event EventTick
  (params (DeltaSeconds :type Float%20%28single-precision%29)))

(fn ConstructionScript
  (bind _boulder (Variables|Default|GetBoulder))
  (bind _boulder_2 (Variables|Default|GetBoulder))
  (bind _box (Variables|Default|GetBox))
  (bind _box_2 (Variables|Default|GetBox))
  (bind _boulder_3 (Variables|Default|GetBoulder))
  (bind _boulder_4 (Variables|Default|GetBoulder))
  (switch Utilities|FlowControl|Switch|SwitchonEnum_BoulderType (Variables|Default|GetBoulderType)
    (:NewEnumerator0
      (Components|StaticMesh|SetStaticMesh _boulder "/Game/Meshes/Environment/Stylized/Organic/SM_Cliff_001.SM_Cliff_001")
      (Rendering|Material|SetMaterial _boulder_3 0 "/Game/Materials/Instances/Stylized/MI_Cliff_001.MI_Cliff_001")
      (Components|Box|SetBoxExtent _box "850.000000,400.000000,350.000000" true))
    (:NewEnumerator1
      (Components|StaticMesh|SetStaticMesh _boulder "/Game/Meshes/Environment/Stylized/Organic/SM_Cliff_002.SM_Cliff_002")
      (Rendering|Material|SetMaterial _boulder_3 0 "/Game/Materials/Instances/Stylized/MI_Cliff_002.MI_Cliff_002")
      (Components|Box|SetBoxExtent _box "250.000000,350.000000,250.000000" true))
    (:NewEnumerator2
      (Components|StaticMesh|SetStaticMesh _boulder_2 "/Game/Meshes/Environment/Stylized/Organic/SM_Cliff_003.SM_Cliff_003")
      (Rendering|Material|SetMaterial _boulder_4 0 "/Game/Materials/Instances/Stylized/MI_Cliff_003.MI_Cliff_003")
      (Components|Box|SetBoxExtent _box_2 "250.000000,350.000000,250.000000" true))
    (:NewEnumerator3
      (Components|StaticMesh|SetStaticMesh _boulder_2 "/Game/Meshes/Environment/Stylized/Organic/SM_RockPile_001.SM_RockPile_001")
      (Rendering|Material|SetMaterial _boulder_4 0 "/Game/Materials/Instances/Stylized/MI_RockPile_001.MI_RockPile_001")
      (Components|Box|SetBoxExtent _box_2 "300.000000,200.000000,200.000000" true))))