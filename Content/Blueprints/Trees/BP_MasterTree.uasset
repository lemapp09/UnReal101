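; BP_MasterTree is a tree actor, named as the master tree Blueprint, that carries a wood value and makes a collapse sound on impact.
; The Construction Script sorts the static mesh's world X scale into three tiers to set WoodValue, so larger trees are worth more wood.
; A hit on the Box component plays the Collapse02 sound at the actor's location, with no filter or repeat guard.
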(event OnComponentHit(Box)
  (params (HitComponent :type Primitive%20Component%20Object%20Reference) (OtherActor :type Actor%20Object%20Reference) (OtherComp :type Primitive%20Component%20Object%20Reference) (NormalImpulse :type Vector :default "0, 0, 0") (Hit :type Hit%20Result%20Structure%20%28by%20ref%29))
  (Audio|PlaySoundatLocation "/Game/StarterContent/Audio/Collapse02.Collapse02" (Transformation|GetActorLocation) "0, 0, 0" (Variables|Default|GetVolumeMultiplier) (Variables|Default|GetPitchMultiplier) (Variables|Default|GetStartTime) 0 0 0 0))

(event EventBeginPlay)

(event Collision|EventActorBeginOverlap
  (params (OtherActor :type Actor%20Object%20Reference)))

(event EventTick
  (params (DeltaSeconds :type Float%20%28single-precision%29)))

(fn ConstructionScript
  (bind _staticmesh (Variables|Default|GetStaticMesh))
  (bind _returnvalue (Transformation|GetWorldScale _staticmesh))
  (bind _x (Math|Vector|BreakVector _returnvalue))
  (if (> _x 0.75)
    (Variables|Default|SetWoodValue 3)
    (elif (> _x 0.5)
      (Variables|Default|SetWoodValue 2)
      (else
        (Variables|Default|SetWoodValue 1)))))