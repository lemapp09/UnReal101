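; BP_PreviewActor is a preview actor that displays a static mesh with an overlay showing whether a spawn is valid.
; Its events set the preview mesh's collision mode, swap the displayed mesh, apply a valid or invalid overlay material, and set slot 0 to an indexed default material.
; The file holds no placement or validation logic, and the construction script is empty.
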(event Custom|SwitchPreviewMesh
  (Components|StaticMesh|SetStaticMesh (Variables|Default|GetSM_PreviewMesh) (Variables|Default|GetNewMesh)))

(event Custom|Switch%20Materials
  (if (Variables|Default|GetisValidSpawn)
    (Rendering|Material|SetOverlayMaterial (Variables|Default|GetSM_PreviewMesh) (Variables|Default|GetvalidMaterial) :!class /Script/Engine.MeshComponent)
    (else
      (Rendering|Material|SetOverlayMaterial (Variables|Default|GetSM_PreviewMesh) (Variables|Default|GetinvalidMaterial) :!class /Script/Engine.MeshComponent))))

(event Custom|SwitchCollisionType
  (Collision|SetCollisionEnabled (Variables|Default|GetSM_PreviewMesh) (Variables|Default|GetcollisionType)))

(event Custom|SetDefaultMaterial
  (Rendering|Material|SetMaterial (Variables|Default|GetSM_PreviewMesh) 0 (Utilities|Array|Get(acopy) (Variables|Default|GetdefaultMaterials) (Variables|Default|GetdefaultMaterialIndex))))

(fn ConstructionScript)