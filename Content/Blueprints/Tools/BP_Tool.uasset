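; BP_Tool is a hand tool (mallet, hatchet or pickaxe) that the first-person player can pick up and drop.
; Construction sets the mesh from ToolType and records its starting transform.
; The PlayerDetect overlap stores or clears the player reference, which gates the pick-up/drop input.
; A FlipFlop alternates between attaching to the player's right-hand socket and detaching, returning the mesh to its starting transform.
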(event OnComponentBeginOverlap(PlayerDetect)
  (params (OverlappedComponent :type Primitive%20Component%20Object%20Reference) (OtherActor :type Actor%20Object%20Reference) (OtherComp :type Primitive%20Component%20Object%20Reference) (OtherBodyIndex :type Integer) (bFromSweep :type Boolean) (SweepResult :type Hit%20Result%20Structure%20%28by%20ref%29))
  ;[1 1 1] Player Overlaps Tool
  (bind _asbp_first_person_character (Utilities|Casting|CastToBP_FirstPersonCharacter OtherActor))
  (Variables|Default|SetPlayerRef _asbp_first_person_character))

(event OnComponentEndOverlap(PlayerDetect)
  (params (OverlappedComponent :type Primitive%20Component%20Object%20Reference) (OtherActor :type Actor%20Object%20Reference) (OtherComp :type Primitive%20Component%20Object%20Reference) (OtherBodyIndex :type Integer))
  ;[1 1 1] Player Leaves Overlap of Tool
  (Utilities|Casting|CastToBP_FirstPersonCharacter OtherActor)
  (Variables|Default|SetPlayerRef 0))

(event Input|EnhancedActionEvents|EnhancedInputActionIA_PickUp_Drop
  (params (ActionValue :type Boolean) (ElapsedSeconds :type Float%20%28double-precision%29) (TriggeredSeconds :type Float%20%28double-precision%29) (InputAction :type Input%20Action%20Object%20Reference :default "/Game/FirstPerson/Input/Actions/IA_PickUp_Drop.IA_PickUp_Drop"))
  (Utilities|IsValid (Variables|Default|GetPlayerRef)
    (:Is%20Valid
      (Utilities|FlowControl|FlipFlop
        (:A
          (Transformation|AttachComponentToComponent (Variables|/Game/FirstPerson/Blueprints/BP_FirstPersonCharacter.BP_FirstPersonCharacter_C|GetFirstPersonMesh (Variables|Default|GetPlayerRef)) "RightHandSocket" "SnapToTarget" "SnapToTarget" "KeepRelative" true))
        (:B
          (Transformation|DetachFromActor "KeepWorld" "KeepWorld" "KeepWorld")
          (Transformation|SetWorldTransform (Variables|Default|GetTool_Mesh) (Variables|Default|GetStartingLocation) false false))))))

(event EventBeginPlay)

(event Collision|EventActorBeginOverlap
  (params (OtherActor :type Actor%20Object%20Reference)))

(event EventTick
  (params (DeltaSeconds :type Float%20%28single-precision%29)))

(fn ConstructionScript
  (Variables|Default|SetStartingLocation (Transformation|GetWorldTransform (Variables|Default|GetTool_Mesh)))
  (switch Utilities|FlowControl|Switch|SwitchonE_ToolType (Variables|Default|GetToolType)
    (:NewEnumerator0
      (Components|StaticMesh|SetStaticMesh (Variables|Default|GetTool_Mesh) "/Game/Meshes/Tools/Polygonal/SM_Poly_Mallet.SM_Poly_Mallet"))
    (:NewEnumerator1
      (Components|StaticMesh|SetStaticMesh (Variables|Default|GetTool_Mesh) "/Game/Meshes/Tools/Polygonal/SM_Polygonal_Hatchet.SM_Polygonal_Hatchet"))
    (:NewEnumerator2
      (Components|StaticMesh|SetStaticMesh (Variables|Default|GetTool_Mesh) "/Game/Meshes/Tools/Polygonal/SM_Polygonal_Pickaxe.SM_Polygonal_Pickaxe"))))